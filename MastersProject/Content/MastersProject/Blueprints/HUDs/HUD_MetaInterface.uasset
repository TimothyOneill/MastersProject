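; HUD that draws directional markers around screen centre for Asteroid and A_Waypoint actors within DetectionRadius of the player, using a separate material for each type.
; DrawHUD finds both actor classes every frame and passes those in range to DrawInterface.
; Each marker is rotated around the centre by the world bearing to its actor minus pawn yaw.
; DrawSmartTexture draws it larger as distance shrinks, up to a capped scale.
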(event EventDrawHUD
  (params (SizeX :type Integer) (SizeY :type Integer))
  (bind _returnvalue (Math|Conversions|ToFloat(Integer) SizeX))
  (bind _returnvalue_2 (Math|Conversions|ToFloat(Integer) SizeY))
  (Variables|Default|SetMaterialToDraw "/Game/MastersProject/Materials/M_Meta_Interface.M_Meta_Interface")
  (bind _outactors (Actor|GetAllActorsOfClass 0 "/Script/MastersProject.Asteroid"))
  (for _array_element _outactors
    (bind _actor (Utilities|IsDetectedActorinRange _array_element)
      (:InRange
        (CallFunction|DrawInterface 256.0 _returnvalue _returnvalue_2 _actor))))
  (Variables|Default|SetMaterialToDraw "/Game/MastersProject/Materials/M_Meta_WayPoint_Interface.M_Meta_WayPoint_Interface")
  (bind _outactors_2 (Actor|GetAllActorsOfClass 0 "/Game/MastersProject/Blueprints/Actors/A_Waypoint.A_Waypoint_C"))
  (for _array_element_2 _outactors_2
    (bind _actor_2 (Utilities|IsDetectedActorinRange _array_element_2)
      (:InRange
        (CallFunction|DrawInterface 256.0 _returnvalue _returnvalue_2 _actor_2)))))

(event EventBeginPlay)

(event EventActorBeginOverlap
  (params (OtherActor :type Actor%20Object%20Reference)))

(event EventTick
  (params (DeltaSeconds :type Float%20%28single-precision%29)))

(fn ConstructionScript)

(fn DrawSmartTexture
  (params (XPos :type Float%20%28single-precision%29) (YPos :type Float%20%28single-precision%29) (Width :type Float%20%28single-precision%29) (Height :type Float%20%28single-precision%29) (IdealScreenSize :type Vector%202D%20Structure) (Material :type Material%20Object%20Reference) (Rotation :type Float%20%28single-precision%29))
  (bind (_xpos _ypos _scalewidth _scaleheight) (CallFunction|GetAdjustedScreenPOSandSize XPos YPos Width Height IdealScreenSize))
  (Canvas|DrawMaterial Material _xpos _ypos _scalewidth _scaleheight 0.0 1.0 1.0 1.0 (Math|Float|Min(Float) (/ 1e+03 (Variables|Default|GetCurrentAsteroidDist)) 2.0) false Rotation))

(fn GetAdjustedScreenPOSandSize
  (params (XPOSin :type Float%20%28single-precision%29) (YPOSin :type Float%20%28single-precision%29) (Width :type Float%20%28single-precision%29) (Height :type Float%20%28single-precision%29) (IdealScreenSize :type Vector%202D%20Structure))
  (bind (_x _y) (Math|Vector2D|BreakVector2D IdealScreenSize))
  (bind _screendimensions (Variables|Default|GetScreenDimensions))
  (bind (_x_2 _y_2) (Math|Vector2D|BreakVector2D _screendimensions))
  (bind _returnvalue (/ _y_2 _y))
  (bind _returnvalue_2 (/ _x_2 _x))
  (return (* XPOSin _returnvalue_2) (* YPOSin _returnvalue) (* Width _returnvalue_2) (* Height _returnvalue) _returnvalue_2 _returnvalue))

(fn DrawInterface
  (params (InterfaceSize :type Float%20%28single-precision%29) (XPos :type Float%20%28single-precision%29) (YPos :type Float%20%28single-precision%29) (ActorToDraw :type Actor%20Object%20Reference))
  (LocalVariables|SetStartX XPos)
  (LocalVariables|SetStartY YPos)
  (bind _angleradians (CallFunction|GetMarkerRotation ActorToDraw))
  (bind _newpoint (CallFunction|RotatePoint (Math|Vector2D|MakeVector2D (/ (LocalVariables|GetStartX) 2.0) (- (/ (LocalVariables|GetStartY) 2.0) InterfaceSize)) (/ (Math|Vector2D|MakeVector2D (LocalVariables|GetStartX) (LocalVariables|GetStartY)) 2.0) (+ _angleradians (Math|Trig|DegreesToRadians (* (.Yaw (Math|Rotator|BreakRotator (Transformation|GetActorRotation (Game|Player|GetPlayerPawn 0)))) -1.0)))))
  (bind (_newx _newy) (CallFunction|GetTempOffset (.X (Math|Vector2D|BreakVector2D _newpoint)) (.Y (Math|Vector2D|BreakVector2D _newpoint))))
  (CallFunction|DrawSmartTexture _newx _newy 32.0 32.0 (Variables|Default|GetScreenDimensions) (Variables|Default|GetMaterialToDraw) (Math|Trig|RadiansToDegrees (+ _angleradians (Math|Trig|DegreesToRadians (* (.Yaw (Math|Rotator|BreakRotator (Transformation|GetActorRotation (Game|Player|GetPlayerPawn 0)))) -1.0))))))

(fn GetTempOffset
  (params (XOffset :type Float%20%28single-precision%29) (YOffset :type Float%20%28single-precision%29))
  (return (+ XOffset (Variables|Default|GetTempXOffset)) (+ YOffset (Variables|Default|GetTemp%20YOffset))))

(fn RotatePoint
  (params (PointToRotate :type Vector%202D%20Structure) (CentrePoint :type Vector%202D%20Structure) (AngleInRad :type Float%20%28single-precision%29))
  (bind (_x _y) (Math|Vector2D|BreakVector2D CentrePoint))
  (bind (_x_2 _y_2) (Math|Vector2D|BreakVector2D PointToRotate))
  (return (Math|Vector2D|MakeVector2D (+ (- (* (Math|Trig|Cos(Radians) AngleInRad) (- _x_2 _x)) (* (Math|Trig|Sin(Radians) AngleInRad) (- _y_2 _y))) _x) (+ _y (+ (* (Math|Trig|Sin(Radians) AngleInRad) (- _x_2 _x)) (* (Math|Trig|Cos(Radians) AngleInRad) (- _y_2 _y)))))))

(fn GetMarkerRotation
  (params (Actor :type Actor%20Object%20Reference))
  (bind _returnvalue (Game|Player|GetPlayerPawn 0))
  (bind _returnvalue_2 (Transformation|GetActorLocation Actor))
  (bind (_x _y) (Math|Vector|BreakVector _returnvalue_2))
  (bind _returnvalue_3 (Transformation|GetActorLocation _returnvalue))
  (bind (_x_2 _y_2) (Math|Vector|BreakVector _returnvalue_3))
  (return (Math|Trig|Atan2(Radians) (- _y _y_2) (- _x _x_2))))