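; Non-diegetic HUD that draws a player-centred radar showing asteroids and waypoints within RadarRadius.
; Each draw, it scans all actors of both classes, converts in-range positions to radar space and rotates them by negated player yaw, keeping the player's heading up.
; Materials are drawn through a helper that scales position and size from a 1080p reference.
; With a head-mounted display enabled, the radar is halved and offset for the Oculus.
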(event EventDrawHUD
  (params (SizeX :type Integer) (SizeY :type Integer))
  (bind _occlusscreendimensions (Variables|Default|GetOcclusScreenDimensions))
  (bind (_x _y) (Math|Vector2D|BreakVector2D _occlusscreendimensions))
  (if (Class|HeadMountedDisplayFunctionLibrary|IsHeadMountedDisplayEnabled)
    ;[1 1 1] If the Oculus is in use we need to shrink the size of the interface due to the smaller resolution, also we need to change its position
    (Variables|Default|SetTempXOffset 1.5e+02)
    (Variables|Default|SetTempYOffset -4e+02)
    (CallFunction|DrawRadar (/ (Variables|Default|GetRadarSize) 2.0) _x _y)
    (else
      (CallFunction|DrawRadar (Variables|Default|GetRadarSize) (Math|Conversions|ToFloat(Integer) SizeX) (Math|Conversions|ToFloat(Integer) SizeY)))))

(fn ConstructionScript)

(fn DrawSmartTexture
  (params (XPos :type Float%20%28single-precision%29) (YPos :type Float%20%28single-precision%29) (Width :type Float%20%28single-precision%29) (Height :type Float%20%28single-precision%29) (IdealScreenSize :type Vector%202D%20Structure) (Material :type Material%20Object%20Reference))
  ;[1 1 1] Correctly alters the position of the interface if the screen is resized
  (bind (_xpos _ypos _scale_width _scale_height) (CallFunction|GetAdjustedScreenPOSandSize XPos YPos Width Height IdealScreenSize))
  (Class|HUD|DrawMaterialSimple Material _xpos _ypos _scale_width _scale_height 1.0 false))

(fn GetAdjustedScreenPOSandSize
  (params (XPOSIn :type Float%20%28single-precision%29) (YPOSin :type Float%20%28single-precision%29) (Width :type Float%20%28single-precision%29) (Height :type Float%20%28single-precision%29) (IdealScreenSize :type Vector%202D%20Structure))
  (bind (_x _y) (Math|Vector2D|BreakVector2D IdealScreenSize))
  (bind _screendimensions (Variables|Default|GetScreenDimensions))
  (bind (_x_2 _y_2) (Math|Vector2D|BreakVector2D _screendimensions))
  (bind _returnvalue (/ _y_2 _y))
  (bind _returnvalue_2 (/ _x_2 _x))
  ;[1 1 1] Gets a ratio of the current screen size to the ideal screen sizes and scales the positions accordingly.
  (return (* XPOSIn _returnvalue_2) (* YPOSin _returnvalue) (* Width _returnvalue_2) (* Height _returnvalue) _returnvalue_2 _returnvalue))

(fn DrawRadar
  (params (RadarSize :type Vector%202D%20Structure) (XPos :type Float%20%28single-precision%29) (YPos :type Float%20%28single-precision%29))
  (bind (_x _y) (Math|Vector2D|BreakVector2D RadarSize))
  ;[1 1 1] Draws the contents of the interface
  (LocalVariables|SetStart%20X XPos)
  (LocalVariables|SetStart%20Y YPos)
  (bind (_new_x _new_y) (CallFunction|GetTempOffset 0.0 0.0))
  (CallFunction|DrawSmartTexture _new_x _new_y _x _y "(X=1920.000000,Y=1080.000000)" (Variables|Default|GetRadar))
  (Variables|Default|SetMarkerMaterial "/Game/MastersProject/Materials/M_Radar_Dot.M_Radar_Dot")
  (bind _outactors (Actor|GetAllActorsOfClass 0 "/Script/MastersProject.Asteroid"))
  (for _array_element _outactors
    (bind _actor (Utilities|IsDetectedActorinRange _array_element)
      (:InRange
        (CallFunction|DrawMarker _actor RadarSize))))
  (Variables|Default|SetMarkerMaterial "/Game/MastersProject/Materials/M_Radar_WayPoint_Interface.M_Radar_WayPoint_Interface")
  (bind _outactors_2 (Actor|GetAllActorsOfClass 0 "/Game/MastersProject/Blueprints/Actors/A_Waypoint.A_Waypoint_C"))
  (for _array_element_2 _outactors_2
    (bind _actor_2 (Utilities|IsDetectedActorinRange _array_element_2)
      (:InRange
        (CallFunction|DrawMarker _actor_2 RadarSize))))
  (bind (_new_x_2 _new_y_2) (CallFunction|GetTempOffset (/ _x 2.0) (/ _y 2.0)))
  (CallFunction|DrawSmartTexture (+ _new_x_2 -16.0) (+ _new_y_2 -16.0) 32.0 32.0 "(X=1920.000000,Y=1080.000000)" (Variables|Default|GetPlayerMark)))

(fn GetTempOffset
  (params (XOffset :type Float%20%28single-precision%29) (YOffset :type Float%20%28single-precision%29))
  ;[1 1 1] Returns the Values of the temp offset variables.
  (return (+ XOffset (Variables|Default|GetTempXOffset)) (+ YOffset (Variables|Default|GetTempYOffset))))

(fn GetRadarPosition
  (params (DetectedActor :type Actor%20Object%20Reference) (RadarSize :type Vector%202D%20Structure))
  (bind _returnvalue (Game|Player|GetPlayerPawn 0))
  (bind _returnvalue_2 (Transformation|GetActorLocation DetectedActor))
  (bind (_x _y) (Math|Vector2D|BreakVector2D RadarSize))
  (bind _radarradius (Variables|Default|GetRadarRadius))
  (bind _returnvalue_3 (Transformation|GetActorLocation _returnvalue))
  (bind _returnvalue_4 (/ _x 2.0))
  (bind _returnvalue_5 (/ _y 2.0))
  (bind _returnvalue_6 (- _returnvalue_3 _returnvalue_2))
  (bind (_x_2 _y_2) (Math|Vector|BreakVector _returnvalue_6))
  ;[1 1 1] Gets the relative x,y position of the supplied actor from the player
  (return (Math|Vector2D|MakeVector2D (+ (* (/ (* _y_2 -1.0) _radarradius) _returnvalue_5) _returnvalue_5) (+ (* (/ _x_2 _radarradius) _returnvalue_4) _returnvalue_4)) (Math|Vector2D|MakeVector2D _returnvalue_4 _returnvalue_5)))

(fn GetRadarRotation
  ;[1 1 1] Gets rotation so the interface allways shows what is in front of the player as north.
  (return (Math|Trig|DegreesToRadians (* (.Yaw (Math|Rotator|BreakRotator (Transformation|GetActorRotation (Game|Player|GetPlayerPawn 0)))) -1.0))))

(fn RotatePoint
  (params (PointToRotate :type Vector%202D%20Structure) (CenterPoint :type Vector%202D%20Structure) (AngleInRad :type Float%20%28single-precision%29))
  (bind (_x _y) (Math|Vector2D|BreakVector2D CenterPoint))
  (bind (_x_2 _y_2) (Math|Vector2D|BreakVector2D PointToRotate))
  ;[1 1 1] Rotates the markers position correctly around the interface
  (return (Math|Vector2D|MakeVector2D (+ (- (* (Math|Trig|Cos(Radians) AngleInRad) (- _x_2 _x)) (* (Math|Trig|Sin(Radians) AngleInRad) (- _y_2 _y))) _x) (+ _y (+ (* (Math|Trig|Sin(Radians) AngleInRad) (- _x_2 _x)) (* (Math|Trig|Cos(Radians) AngleInRad) (- _y_2 _y)))))))

(fn DrawMarker
  (params (MarkerToDraw :type Actor%20Object%20Reference) (RadarSize :type Vector%202D%20Structure))
  ;[1 1 1] Draws the supplied marker for  given entity on the interface
  (bind (_radarposition _radarcenter) (CallFunction|GetRadarPosition MarkerToDraw RadarSize))
  (bind _radarrotation (CallFunction|GetRadarRotation))
  (bind _newpoint (CallFunction|RotatePoint _radarposition _radarcenter _radarrotation))
  (bind (_new_x _new_y) (CallFunction|GetTempOffset (.X (Math|Vector2D|BreakVector2D _newpoint)) (.Y (Math|Vector2D|BreakVector2D _newpoint))))
  (CallFunction|DrawSmartTexture (+ _new_x -16.0) (+ _new_y -16.0) 32.0 32.0 "(X=1920.000000,Y=1080.000000)" (Variables|Default|GetMarkerMaterial)))